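; Turn-based mode Blueprint that handles player defeat and level transitions, with no turn logic of its own.
; On BeginPlay it creates a hidden WEP_DefeatWidget and binds to the BPT_HeroCharacter death event, revealing the widget after a short delay when the player dies.
; Helper functions store the next level's name, open that level, or restart the current one by name.
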(event Custom|ShowGameOverScreen
  (Utilities|FlowControl|Delay 2.0)
  (CallFunction|GameOverScreen))

(event EventBeginPlay
  (bind _returnvalue (UserInterface|CreateWidget "/Game/Widgets/WEP_DefeatWidget.WEP_DefeatWidget_C"))
  (bind _output_get (Variables|Default|SetDefeatWidget _returnvalue))
  (UserInterface|Viewport|AddtoViewport _output_get 0)
  (Widget|SetVisibility _output_get "Hidden")
  (bind _asbpt_hero_character (Utilities|Casting|CastToBPT_HeroCharacter (Game|GetPlayerCharacter 0)))
  (EventDispatchers|BindEventtoOnPlayerDeath _asbpt_hero_character (delegate Custom|ShowGameOverScreen)))

(fn ConstructionScript)

(fn SetNextLevel
  (params (LevelToLoad :type Name))
  (Variables|Default|SetLevelToLoad LevelToLoad))

(fn OpenNextLevel
  (Game|OpenLevel(byName) (Variables|Default|GetLevelToLoad)))

(fn RestartLevel
  (bind _returnvalue (Game|GetCurrentLevelName true))
  (Game|OpenLevel(byName) (Utilities|String|StringToName _returnvalue)))

(fn GameOverScreen
  (Widget|SetVisibility (Variables|Default|GetDefeatWidget) "Visible"))