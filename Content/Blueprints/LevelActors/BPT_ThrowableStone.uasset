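; A throwable stone actor that flies at a target and creates a noise when it lands on a node.
; ThrowStone sets the launch velocity and makes the projectile movement home in on the given actor.
; When its sphere overlaps a BPT_Node, it re-enables node clicking on the player hero, has the hero report noise, plays an impact sound and destroys itself.
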(event OnComponentBeginOverlap(SphereCollider)
  (params (OverlappedComponent :type Primitive%20Component%20Object%20Reference) (OtherActor :type Actor%20Object%20Reference) (OtherComp :type Primitive%20Component%20Object%20Reference) (OtherBodyIndex :type Integer) (bFromSweep :type Boolean) (SweepResult :type Hit%20Result%20Structure%20%28by%20ref%29))
  (Utilities|Casting|CastToBPT_Node OtherActor)
  (bind _asbpt_hero_character (Utilities|Casting|CastToBPT_HeroCharacter (Game|GetPlayerCharacter 0)))
  (Variables|/Game/Blueprints/Characters/Hero/BPT_HeroCharacter.BPT_HeroCharacter_C|SetCanClickNode _asbpt_hero_character true)
  (Default|ReportNoise _asbpt_hero_character)
  (Audio|PlaySound2D "/Game/SoundFX/Pickups/StoneImpact.StoneImpact" 1.0 1.0 0.0 0 0)
  (Actor|DestroyActor))

(event Custom|Throw%20Stone
  (params (Actor :type Actor%20Object%20Reference) (Velocity :type Vector))
  (bind _projectilemovement (Variables|Default|GetProjectileMovement))
  (Variables|/Script/Engine.ProjectileMovementComponent|SetbIsHomingProjectile _projectilemovement true)
  (Variables|/Script/Engine.ProjectileMovementComponent|SetHomingTargetComponent _projectilemovement (Variables|/Script/Engine.Actor|GetRootComponent Actor))
  (Variables|/Script/Engine.MovementComponent|SetVelocity _projectilemovement Velocity)
  (Variables|/Script/Engine.ProjectileMovementComponent|SetHomingAccelerationMagnitude _projectilemovement 2e+03))

(fn ConstructionScript)