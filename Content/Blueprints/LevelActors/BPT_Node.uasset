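; BPT_Node is a board node actor for a turn-based level, configurable as an end node, trap or teleport.
; Construction script flags reveal side panels, teleport FX and end-node decoration.
; Hero overlap stops movement and re-enables node clicking; end nodes set the next level and show the victory widget, while traps raise spikes on a linked TrapNode.
; End overlap hides its own spikes; the trap's enemy cast leads nowhere.
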(event OnComponentBeginOverlap(BoxCollider)
  (params (OverlappedComponent :type Primitive%20Component%20Object%20Reference) (OtherActor :type Actor%20Object%20Reference) (OtherComp :type Primitive%20Component%20Object%20Reference) (OtherBodyIndex :type Integer) (bFromSweep :type Boolean) (SweepResult :type Hit%20Result%20Structure%20%28by%20ref%29))
  (bind _trapnode (Variables|Default|GetTrapNode))
  (bind _asbpt_hero_character (Utilities|Casting|CastToBPT_HeroCharacter OtherActor))
  (Variables|/Game/Blueprints/Characters/Hero/BPT_HeroCharacter.BPT_HeroCharacter_C|SetIsMoving _asbpt_hero_character false)
  (Variables|/Game/Blueprints/Characters/Hero/BPT_HeroCharacter.BPT_HeroCharacter_C|SetCanClickNode _asbpt_hero_character true)
  (Utilities|FlowControl|Sequence
    (:then_0
      (if (Variables|Default|GetisEndNode)
        (bind _asbtp_turn_based_mode (Utilities|Casting|CastToBTP_TurnBasedMode (Game|GetGameMode)))
        (Default|SetNextLevel _asbtp_turn_based_mode (Variables|Default|GetLevelName))
        (bind _returnvalue (UserInterface|CreateWidget "/Game/Widgets/WEP_VictoryWidget.WEP_VictoryWidget_C" (Game|GetPlayerController 0)))
        (UserInterface|Viewport|AddtoViewport _returnvalue 0)))
    (:then_1
      (if (Variables|Default|GetisTrap)
        (Utilities|IsValid _trapnode
          (:Is%20Valid
            (CallFunction|ShowSpikes _trapnode)
            (Utilities|Casting|CastToBPT_EnemyBase (Utilities|Array|Get(acopy) (Collision|GetOverlappingActors (Variables|BPT_Node_C|GetBoxCollider _trapnode) 0 :!class /Script/Engine.PrimitiveComponent)))))))))

(event OnComponentEndOverlap(BoxCollider)
  (params (OverlappedComponent :type Primitive%20Component%20Object%20Reference) (OtherActor :type Actor%20Object%20Reference) (OtherComp :type Primitive%20Component%20Object%20Reference) (OtherBodyIndex :type Integer))
  (CallFunction|HideSpikes))

(fn ConstructionScript
  (Utilities|FlowControl|Sequence
    (:then_0
      (if (Variables|Default|GetShowPanel1)
        (Rendering|SetVisibility (Variables|Default|GetPanel1) true false)))
    (:then_1
      (if (Variables|Default|GetShowPanel2)
        (Rendering|SetVisibility (Variables|Default|GetPanel2) true false)))
    (:then_2
      (if (Variables|Default|GetShowPanel3)
        (Rendering|SetVisibility (Variables|Default|GetPanel3) true false)))
    (:then_3
      (if (Variables|Default|GetShowPanel4)
        (Rendering|SetVisibility (Variables|Default|GetPanel4) true false)))
    (:then_4
      (if (Variables|Default|GetisTeleport)
        (Rendering|SetVisibility (Variables|Default|GetTeleport_FX) true false)))
    (:then_5
      (if (Variables|Default|GetisEndNode)
        (Rendering|SetVisibility (Variables|Default|GetDecoMesh) true false)))))

(fn ShowSpikes
  (Rendering|SetVisibility (Variables|Default|GetSpikeMesh) true false))

(fn HideSpikes
  (Rendering|SetVisibility (Variables|Default|GetSpikeMesh) false false))