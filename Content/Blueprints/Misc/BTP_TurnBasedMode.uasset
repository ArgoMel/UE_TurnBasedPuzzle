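; Turn-based mode Blueprint, apparently a game mode, that handles player defeat and level transitions.
; On BeginPlay it creates a collapsed defeat widget and binds to the hero character's player death event.
; On death it waits briefly, then makes the defeat widget visible.
; Separate functions store the next level's name, open that level, or restart the current one by name.
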(event Custom|ShowGameOverScreen
  (Utilities|FlowControl|Delay 2.0)
  (CallFunction|GameOverScreen))

(event EventBeginPlay
  (bind _returnvalue (UserInterface|CreateWidget "/Game/Widgets/WEP_DefeatWidget.WEP_DefeatWidget_C" (Game|GetPlayerController 0)))
  (bind _output_get (Variables|Default|SetDefeatWidget _returnvalue))
  (Widget|SetVisibility _output_get "Collapsed")
  (UserInterface|Viewport|AddtoViewport _output_get 0)
  (bind _asbpt_hero_character (Utilities|Casting|CastToBPT_HeroCharacter (Game|GetPlayerCharacter 0)))
  (EventDispatchers|BindEventtoOnPlayerDeath _asbpt_hero_character (delegate Custom|ShowGameOverScreen)))

(event EventTick
  (params (DeltaSeconds :type Float%20%28single-precision%29)))

(fn ConstructionScript)

(fn SetNextLevel
  (params (LevelToLoad :type Name))
  (Variables|Default|SetLevelToLoad LevelToLoad))

(fn OpenNextLevel
  (Game|OpenLevel(byName) (Variables|Default|GetLevelToLoad)))

(fn RestartLevel
  (bind _returnvalue (Game|GetCurrentLevelName true))
  (Game|OpenLevel(byName) (Utilities|String|StringToName _returnvalue)))

(fn GameOverScreen
  (Widget|SetVisibility (Variables|Default|GetDefeatWidget) "Visible"))